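; Crosshair Blueprint that draws a debug point in front of the player camera to serve as an aiming marker.
; Every Tick it runs a visibility line trace from just above the camera along its forward vector for InteractionDistance, ignoring the player pawn.
; The point sits along that ray at 90% of the hit distance, clamped to at most one unit from the trace start.
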(event `self.ReceiveTick`
  (params (DeltaSeconds :type "Float (single-precision)"))
  (bind _returnvalue (`GameplayStatics.GetPlayerCameraManager` 0))
  (set `self.Crosshair Start Point` (+ (`self.K2_GetActorLocation` _returnvalue) (0.0 0.0 10.0)))
  (set `self.Crosshair Vector` (`KismetMathLibrary.Normal` (`KismetMathLibrary.Conv_RotatorToVector` (`self.K2_GetActorRotation` _returnvalue))))
  (bind _outhit (`KismetSystemLibrary.LineTraceSingle` (`self.Crosshair Start Point`) (+ (`self.Crosshair Start Point`) (* (`self.Crosshair Vector`) (`self.interaction distance`))) "TraceTypeQuery1" false (`|MakeArray` (`GameplayStatics.GetPlayerPawn` 0) :!type "Actor Object Reference")))
  (`KismetSystemLibrary.DrawDebugPoint` (+ (`self.Crosshair Start Point`) (* (`self.Crosshair Vector`) (`KismetMathLibrary.FClamp` (* (`KismetMathLibrary.VSize` (- (`.Location` (`GameplayStatics.BreakHitResult` _outhit)) (`self.Crosshair Start Point`))) 0.9))))))

(fn `UserConstructionScript`)