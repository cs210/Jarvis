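; EditorCharacter is a gamepad-driven character that moves, looks around and gaze-selects menu items.
; Each tick, a visibility trace along control rotation flags a hit MenuItem_old as gazed and stores it as SelectedMenu.
; When the trace hits nothing, it clears the gaze flag on all MenuItem_old actors.
; The special-right button, labeled as the main menu toggle, only spawns a GroupActor far ahead along the view direction.
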(event `self.ReceiveTick`
  (params (DeltaSeconds :type "Float (single-precision)"))
  (bind _returnvalue (`SceneComponent.K2_GetComponentLocation`))
  ;[1 1 1] raytrace to select objects
  (bind (_outhit _returnvalue_2) (`KismetSystemLibrary.LineTraceSingle` _returnvalue (+ (* (`KismetMathLibrary.GetForwardVector` (`self.GetControlRotation`)) 5000.0) _returnvalue) "TraceTypeQuery1"))
  (if _returnvalue_2
    (bind (_bblockinghit _time _location _normal _impactpoint _impactnormal _physmat _hitactor) (`GameplayStatics.BreakHitResult` _outhit))
    (bind _asmenu_item_old (cast `/Game/Blueprints/Menus/MenuItem_old` _hitactor))
    (set `/Game/Blueprints/Menus/MenuItem_old.isGaze` true _asmenu_item_old)
    (set `self.Selected Menu` _hitactor)
    (`KismetSystemLibrary.PrintString` "hit item")
    (else
      (bind _outactors (`GameplayStatics.GetAllActorsOfClass` "/Game/Blueprints/Menus/MenuItem_old.MenuItem_old_C"))
      (for _array_element _outactors
        (set `/Game/Blueprints/Menus/MenuItem_old.isGaze` false _array_element)))))

(event `Key|Gamepad_Special_Right`
  ;[1 1 1] Toggle main menu
  (:`Pressed`
    (`|SpawnActorFromClass` "/Script/UnrealEd.GroupActor" (`KismetMathLibrary.Conv_VectorToTransform` (+ (* (`KismetMathLibrary.GetForwardVector` (`self.GetControlRotation`)) 5000.0) (`SceneComponent.K2_GetComponentLocation`))))))

(event `InputAxis|MoveForward`
  (params (AxisValue :type "Float (single-precision)"))
  ;[1 1 1] Movement
  ;;[1 1 1] Left Joystick
  (`self.AddMovementInput` (`KismetMathLibrary.Conv_RotatorToVector` (`self.GetControlRotation`)) AxisValue))

(event `InputAxis|TurnRate`
  (params (AxisValue :type "Float (single-precision)"))
  ;[1 1 1] Movement
  ;;[1 1 1] Right Joystick
  (`self.AddControllerYawInput` (* AxisValue (`GameplayStatics.GetWorldDeltaSeconds`) (`self.BaseTurnRate`))))

(event `InputAxis|LookUpRate`
  (params (AxisValue :type "Float (single-precision)"))
  ;[1 1 1] Movement
  ;;[1 1 1] Right Joystick
  (`self.AddControllerPitchInput` (* AxisValue (`GameplayStatics.GetWorldDeltaSeconds`) (`self.BaseTurnRate`))))

(event `InputAxis|MoveRight`
  (params (AxisValue :type "Float (single-precision)"))
  ;[1 1 1] Movement
  ;;[1 1 1] Left Joystick
  (`self.AddMovementInput` (`KismetMathLibrary.GetRightVector` (`self.GetControlRotation`)) AxisValue))

(fn `UserConstructionScript`)