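; Menu item that belongs to a parent Menu and grows when the player gazes at it.
; On BeginPlay it enables player input, stores its default draw size and caches the Menu that owns its attach parent.
; The ToggleMenu input toggles its visibility.
; Each Tick it enlarges the draw size while IsGaze is set, which this graph only reads, and otherwise restores the default.
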(event `self.ReceiveBeginPlay`
  (`self.EnableInput` (`GameplayStatics.GetPlayerController` 0))
  ;[1 1 1] Set Initial Draw size to reference later
  (set `self.Default Draw Size` (`WidgetComponent.GetDrawSize`))
  ;[1 1 1] Set Parent Menu so it's easy to reference
  (bind _asmenu (cast `/Game/Blueprints/Menus/Menu` (`ActorComponent.GetOwner` (`SceneComponent.GetAttachParent`))))
  (set `self.ParentMenu` _asmenu))

(event `InputAction|ToggleMenu`
  (:`Pressed`
    (`SceneComponent.ToggleVisibility` true)))

(event `self.ReceiveTick`
  (params (DeltaSeconds :type "Float (single-precision)"))
  ;[1 1 1] Set increase the scale if looking at the menu item
  (if (`self.IsGaze`)
    (`WidgetComponent.SetDrawSize` (* (`self.Default Draw Size`) 1.2))
    (else
      (`WidgetComponent.SetDrawSize` (`self.Default Draw Size`)))))

(fn `UserConstructionScript`)